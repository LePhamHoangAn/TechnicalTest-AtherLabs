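; BP_Enemy is an AI enemy with a montage-driven sword attack that damages pawns.
; SwordAttack plays the combo montage, while Begin and End SwordTrace events start and clear a fast looping timer that runs DamageTrace.
; DamageTrace sphere-traces between two blade points with debug drawing and applies sword damage, using a DoOnce that resets after a short delay to limit repeat hits.
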(event Custom|Damage%20Trace
  ;[0.15 0.15 0.15 0.5] Sword trace
  (bind (_outhit _returnvalue) (Collision|SphereTraceForObjects (Transformation|GetWorldLocation (Variables|Default|GetStart%20Sword%20Trace%20Pos)) (Transformation|GetWorldLocation (Variables|Default|GetEnd%20Sword%20Trace%20Pos)) 2e+01 (Utilities|Array|MakeArray "ObjectTypeQuery3") false 0 "ForOneFrame"))
  (if _returnvalue
    (Utilities|FlowControl|DoOnce false :!label _label
      (:Completed
        (Game|Damage|ApplyDamage (.HitActor (Collision|BreakHitResult _outhit)) (Variables|Default|GetSwordDamge) 0 0)
        (Utilities|FlowControl|Delay 0.3)
        (goto _label Reset)))))

(event EventBeginSwordTrace
  ;[0.15 0.15 0.15 0.5] Sword trace
  (bind _returnvalue (Utilities|Time|SetTimerbyEvent (delegate Custom|Damage%20Trace) 0.01 true)))

(event EventEndSwordTrace
  ;[0.15 0.15 0.15 0.5] Sword trace
  (if (Utilities|Time|IsValidTimerHandle (stale EventBeginSwordTrace _returnvalue))
    (Utilities|Time|ClearandInvalidateTimerbyHandle (stale EventBeginSwordTrace _returnvalue))))

(fn ConstructionScript)

(fn SwordAttack
  (bind _returnvalue (Animation|PlayAnimMontage "/Game/Sword_Animations/Animations/Sequence/02_Attack/01_Combo_Attack_01/Combo_Attack_01_02_Seq_Montage.Combo_Attack_01_02_Seq_Montage" 1.0 "None"))
  (return _returnvalue))